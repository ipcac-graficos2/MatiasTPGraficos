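; MainPlayer is the player character, which moves relative to camera yaw, jumps, and visually rolls a Sphere component as it travels.
; Axis inputs drive look and movement, while Pause opens a Pause widget, disables player input, shows the cursor and pauses the game.
; Each Tick, horizontal speed scaled by a Ratio accumulates into an angle that sets the sphere's world rotation around the axis perpendicular to velocity.
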(event EventTick
  (params (DeltaSeconds :type Float%20%28single-precision%29))
  (bind _returnvalue (Transformation|GetVelocity))
  (bind (_x _y) (Math|Vector|BreakVector _returnvalue))
  (Variables|Default|SetHorizontalVer (Math|Vector|MakeVector _x _y 0.0))
  (Variables|Default|SetHorizontal%20Speed (Math|Vector|VectorLength (Variables|Default|GetHorizontalVer)))
  (Math|Float|CompareFloat (Variables|Default|GetHorizontal%20Speed) 0.0
    (:>
      (Variables|Default|SetRotation%20Amount (+ (Variables|Default|GetRotation%20Amount) (* (/ (Variables|Default|GetHorizontal%20Speed) (* (Math|Trig|GetPI) (Variables|Default|GetRatio))) (Utilities|Time|GetWorldDeltaSeconds))))
      (Transformation|SetWorldRotation (Variables|Default|GetSphere) (Math|Vector|RotatorfromAxisandAngle (Math|Vector|GetRightVector (Math|Rotator|MakeRotfromX (Math|Vector|Normalize (Variables|Default|GetHorizontalVer)))) (Variables|Default|GetRotation%20Amount)) false false))))

(event Collision|EventHit
  (params (MyComp :type Primitive%20Component%20Object%20Reference) (Other :type Actor%20Object%20Reference) (OtherComp :type Primitive%20Component%20Object%20Reference) (bSelfMoved :type Boolean) (HitLocation :type Vector :default "0, 0, 0") (HitNormal :type Vector :default "0, 0, 0") (NormalImpulse :type Vector :default "0, 0, 0") (Hit :type Hit%20Result%20Structure%20%28by%20ref%29)))

(event Input|ActionEvents|InputActionJump
  (params (Key :type Key%20Structure :default "None"))
  (:Pressed
    (Character|Jump)))

(event Input|ActionEvents|InputActionPause
  (params (Key :type Key%20Structure :default "None"))
  (bind _returnvalue (Game|GetPlayerController 0))
  (:Pressed
    (bind _returnvalue_2 (UserInterface|CreateWidget "/Game/UI/Pause.Pause_C"))
    (UserInterface|Viewport|AddtoViewport _returnvalue_2 0)
    (Input|DisableInput (Game|GetPlayerCharacter 0) _returnvalue)
    (Variables|/Script/Engine.PlayerController|SetbShowMouseCursor _returnvalue true)
    (Game|SetGamePaused true)))

(event Input|AxisEvents|InputAxisLookHor
  (params (AxisValue :type Float%20%28single-precision%29))
  (Pawn|Input|AddControllerYawInput AxisValue))

(event Input|AxisEvents|InputAxisLookVer
  (params (AxisValue :type Float%20%28single-precision%29))
  (Pawn|Input|AddControllerPitchInput AxisValue))

(event Input|AxisEvents|InputAxisFor_Back
  (params (AxisValue :type Float%20%28single-precision%29))
  (Pawn|Input|AddMovementInput (Math|Vector|GetForwardVector (Math|Rotator|MakeRotator 0.0 0.0 (.yaw (Pawn|GetControlRotation :!class /Script/Engine.Pawn)))) AxisValue false))

(event Input|AxisEvents|InputAxisRight_Left
  (params (AxisValue :type Float%20%28single-precision%29))
  (Pawn|Input|AddMovementInput (Math|Vector|GetRightVector (Math|Rotator|MakeRotator 0.0 0.0 (.yaw (Pawn|GetControlRotation :!class /Script/Engine.Pawn)))) AxisValue false))

(fn ConstructionScript)